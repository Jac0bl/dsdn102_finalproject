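; A scoring bumper Blueprint that knocks a Ball away when it hits the cylinder and awards points to the player.
; On a component hit, it applies a velocity-change impulse to the ball's sphere along the negated hit normal, scaled by BounceForce.
; It then casts the player pawn to Paddle and adds PointValue to PlayerPoints, with debug prints along the way.
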(event `self.Cylinder.OnComponentHit`
  (params (HitComponent :type "PrimitiveComponent Object Reference") (OtherActor :type "Actor Object Reference") (OtherComp :type "PrimitiveComponent Object Reference") (NormalImpulse :type "Vector Structure") (Hit :type "HitResult Structure (by ref)"))
  (bind (_bblockinghit _binitialoverlap _time _distance _location _impactpoint _normal) (`GameplayStatics.BreakHitResult` Hit))
  (`KismetSystemLibrary.PrintString` "Hello")
  (bind _asball (cast `/Game/Ball` OtherActor))
  (`KismetSystemLibrary.PrintString` (`KismetStringLibrary.Conv_VectorToString` _normal) true true (struct :`G` 0.66 :`B` 1.0 :`A` 1.0) 20.0)
  (`PrimitiveComponent.AddVelocityChangeImpulseAtLocation` (`/Game/Ball.Sphere` _asball) (* (- (0.0 0.0 0.0) _normal) (`self.bounceForce`)) (0.0 0.0 0.0) "None")
  (`KismetSystemLibrary.PrintString` "3o")
  (bind _aspaddle (cast `/Game/Paddle` (`GameplayStatics.GetPlayerPawn` 0)))
  (set `/Game/Paddle.playerPoints` (+ (`/Game/Paddle.playerPoints` _aspaddle) (`self.pointValue`)) _aspaddle))

(fn `UserConstructionScript`)